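; Player actor for a chess-style board game that lets the user place pieces with the mouse on their turn.
; It finds the ChessBoard and Match at BeginPlay, then updates the board's placement preview every tick during the player's round.
; PlaceChess input places a piece in the player's color if allowed, then switches the round.
; Positions come from a deprojected mouse Visibility trace, falling back to world origin on a miss.
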(event EventBeginPlay
  (bind _returnvalue (Actor|GetActorOfClass "/Script/TicTacToe.ChessBoard"))
  (Variables|Default|SetChessBoard _returnvalue)
  (bind _returnvalue_2 (Actor|GetActorOfClass "/Script/TicTacToe.Match"))
  (Variables|Default|SetMatch _returnvalue_2))

(event Collision|EventActorBeginOverlap
  (params (OtherActor :type Actor%20Object%20Reference)))

(event EventTick
  (params (DeltaSeconds :type Float%20%28single-precision%29))
  (if (Class|Match|IsPlayerRound (Variables|Default|GetMatch))
    (bind _location (CallFunction|GetChessPlaceLocation))
    (Class|ChessBoard|UpdateChessPreviewinChessBoardPosition (Variables|Default|GetChessBoard) _location)))

(event Input|ActionEvents|InputActionPlaceChess
  (params (Key :type Key%20Structure :default "None"))
  (:Pressed
    (if (Class|Match|IsPlayerRound (Variables|Default|GetMatch))
      (bind _location (CallFunction|GetChessPlaceLocation))
      (bind _returnvalue (Class|ChessBoard|CanPlaceChess (Variables|Default|GetChessBoard) _location))
      (if _returnvalue
        (Class|ChessBoard|PlaceChessinChessBoardPosition (Variables|Default|GetChessBoard) _location (Variables|/Script/TicTacToe.Match|GetbPlayerWhite (Variables|Default|GetMatch)))
        (Class|Match|SwitchRound (Variables|Default|GetMatch))))))

(fn ConstructionScript)

(fn GetChessPlaceLocation
  (bind _asplayer_controller (Utilities|Casting|CastToPlayerController (Pawn|GetController)))
  (bind (_outhit _returnvalue) (Collision|LineTraceByChannel (.WorldPosition (Class|GameplayStatics|DeprojectScreentoWorld _asplayer_controller (Math|Vector2D|MakeVector2D (.LocationX (Game|Player|GetMousePosition _asplayer_controller)) (.LocationY (Game|Player|GetMousePosition _asplayer_controller))))) (* (.WorldDirection (Class|GameplayStatics|DeprojectScreentoWorld _asplayer_controller (Math|Vector2D|MakeVector2D (.LocationX (Game|Player|GetMousePosition _asplayer_controller)) (.LocationY (Game|Player|GetMousePosition _asplayer_controller))))) (Variables|Config|GetTraceLength)) "TraceTypeQuery1" false 0 "None"))
  (if _returnvalue
    (return (.Location (Collision|BreakHitResult _outhit)))
    (else
      (return "0, 0, 0"))))