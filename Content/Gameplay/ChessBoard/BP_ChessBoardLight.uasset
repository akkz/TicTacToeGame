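; BP_ChessBoardLight is a chessboard prop actor whose color, emissive look and mesh are configurable per instance.
; Its construction script reuses the Cube component's dynamic material instance, or creates one if absent, then sets its Color and Emissive parameters.
; A valid CustomStaticMesh replaces the Cube's mesh.
; The event graph has no runtime logic.
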(event EventBeginPlay)

(event Collision|EventActorBeginOverlap
  (params (OtherActor :type Actor%20Object%20Reference)))

(event EventTick
  (params (DeltaSeconds :type Float%20%28single-precision%29)))

(fn ConstructionScript
  (bind _cube (Variables|Default|GetCube))
  (bind _customstaticmesh (Variables|Default|GetCustomStaticMesh))
  (bind _returnvalue (Rendering|Material|GetMaterial _cube 0))
  (bind _asmaterial_instance_dynamic (Utilities|Casting|CastToMaterialInstanceDynamic _returnvalue)
    (:then
      _)
    (:CastFailed
      (bind _returnvalue_2 (Rendering|Material|CreateDynamicMaterialInstance (Variables|Default|GetCube) 0 _returnvalue "None" :!class /Script/Engine.PrimitiveComponent))
      (Rendering|Material|SetMaterial (Variables|Default|GetCube) 0 _returnvalue_2)))
  (Rendering|Material|SetVectorParameterValue _asmaterial_instance_dynamic "Color" (Variables|Default|GetColor) :!class /Script/Engine.MaterialInstanceDynamic)
  (Rendering|Material|SetVectorParameterValue _returnvalue_2 "Emissive" (Variables|Default|GetEmissive) :!class /Script/Engine.MaterialInstanceDynamic)
  (Utilities|IsValid _customstaticmesh
    (:Is%20Valid
      (Components|StaticMesh|SetStaticMesh (Variables|Default|GetCube) _customstaticmesh))))