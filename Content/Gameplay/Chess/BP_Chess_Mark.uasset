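; BP_Chess_Mark is a marker actor for the chess gameplay that continuously pulses in size.
; On Tick it sets its uniform actor scale from a cosine of game time, oscillating quickly and subtly just below full size.
; It holds no other logic: BeginPlay and overlap events are disabled, and the construction script only calls its parent.
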(event EventBeginPlay
  (|CallParentFunction) ; This node is disabled and will not be called.\nDrag off pins to build functionality.
)

(event Collision|EventActorBeginOverlap
  (params (OtherActor :type Actor%20Object%20Reference))
  (|CallParentFunction OtherActor) ; This node is disabled and will not be called.\nDrag off pins to build functionality.
)

(event EventTick
  (params (DeltaSeconds :type Float%20%28single-precision%29))
  (|CallParentFunction DeltaSeconds)
  ;[1 1 1] 缩放
  (Transformation|SetActorScale3D (Math|Conversions|ToVector(Float) (+ (* (Math|Trig|Cos(Degrees) (* (Utilities|Time|GetTimeSeconds) 5e+02)) 0.02) 0.98))))

(fn ConstructionScript
  (|CallParentFunction))