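; BP_Chess is a chess-related mesh actor that fades into view after it spawns.
; The construction script ensures the mesh's first material slot holds a dynamic material instance and sets its Opacity parameter to zero.
; From BeginPlay, a looping timer, used instead of Tick, samples DisplayCurve by time since spawn to drive Opacity, then clears itself once the curve reaches full opacity.
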(event Custom|DisplayEvent
  (bind _returnvalue (Utilities|Time|GetTimeSeconds))
  (bind _spawntime (Variables|Default|GetSpawnTime))
  (bind _displaycurve (Variables|Config|GetDisplayCurve))
  (bind _returnvalue_2 (- _returnvalue _spawntime))
  (bind _returnvalue_3 (Math|Curves|GetFloatValue _displaycurve _returnvalue_2))
  (bind _asmaterial_instance_dynamic (Utilities|Casting|CastToMaterialInstanceDynamic (Rendering|Material|GetMaterial (Variables|Default|GetStaticMeshComponent) 0)))
  (Rendering|Material|SetScalarParameterValue _asmaterial_instance_dynamic "Opacity" _returnvalue_3 :!class /Script/Engine.MaterialInstanceDynamic)
  (if (>= _returnvalue_3 1.0)
    (Utilities|Time|ClearandInvalidateTimerbyHandle (Variables|Default|GetDisplayTimer))))

(event EventBeginPlay
  (Variables|Default|SetSpawnTime (Utilities|Time|GetTimeSeconds))
  (bind _returnvalue (Utilities|Time|SetTimerbyEvent (delegate Custom|DisplayEvent) 0.1 true))
  (Variables|Default|SetDisplayTimer _returnvalue))

(event Collision|EventActorBeginOverlap
  (params (OtherActor :type Actor%20Object%20Reference)))

(event EventTick
  (params (DeltaSeconds :type Float%20%28single-precision%29)))

(fn ConstructionScript
  (bind _staticmeshcomponent (Variables|Default|GetStaticMeshComponent))
  (bind _returnvalue (Rendering|Material|GetMaterial _staticmeshcomponent 0))
  (bind _asmaterial_instance_dynamic (Utilities|Casting|CastToMaterialInstanceDynamic _returnvalue)
    (:then
      _)
    (:CastFailed
      (bind _returnvalue_2 (Rendering|Material|CreateDynamicMaterialInstance _staticmeshcomponent 0 _returnvalue "None" :!class /Script/Engine.PrimitiveComponent))
      (Rendering|Material|SetMaterial (Variables|Default|GetStaticMeshComponent) 0 _returnvalue_2)))
  (Rendering|Material|SetScalarParameterValue _returnvalue_2 "Opacity" 0.0 :!class /Script/Engine.MaterialInstanceDynamic))