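; BP_Match is the match actor that handles UI, music and camera feedback across the ready, start and finished phases of a match.
; Each phase event clears existing widgets and shows its own menu, match or results widget.
; In fast mode, Tick raises the looping BGM reference's pitch as round time shrinks, resetting it at match end.
; Round switches on the player's turn trigger a delayed camera shake, scaled inversely to round time.
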(event EventBeginPlay
  (bind _returnvalue (Audio|SpawnSound2D "/Game/Res/BGM.BGM" 1.0 1.0 0.0 0))
  (Variables|Default|SetBGM _returnvalue))

(event Collision|EventActorBeginOverlap
  (params (OtherActor :type Actor%20Object%20Reference)))

(event EventTick
  (params (DeltaSeconds :type Float%20%28single-precision%29))
  (bind _currentroundtime (Variables|Default|GetCurrentRoundTime))
  (bind _returnvalue (Utilities|Operators|Divide 5.0 _currentroundtime 1e+01))
  (bind _returnvalue_2 (+ _returnvalue 0.9))
  (if (Math|Boolean|ANDBoolean (Variables|Default|GetbFastMode) (Class|Match|IsMatchRunning) (> (Variables|Default|GetCurrentRoundTime) 0.0))
    ;[1 1 1] 根据比赛节奏挑战音频
    (if (!= (Variables|/Script/Engine.AudioComponent|GetPitchMultiplier (Variables|Default|GetBGM)) _returnvalue_2)
      (Audio|Components|Audio|SetPitchMultiplier (Variables|Default|GetBGM) _returnvalue_2))))

(event EventOnMatchFinished
  (CallFunction|ClearWidget)
  (bind _returnvalue (UserInterface|CreateWidget "/Game/Gameplay/Match/BP_MatchFinishedWidget.BP_MatchFinishedWidget_C" (Game|GetPlayerController 0)))
  (bind _output_get (Variables|Widgets|SetFinishWidget _returnvalue))
  (UserInterface|Viewport|AddtoViewport _output_get 0)
  (Audio|Components|Audio|SetPitchMultiplier (Variables|Default|GetBGM) 1.0))

(event EventOnMatchStart
  (CallFunction|ClearWidget)
  (bind _returnvalue (UserInterface|CreateWidget "/Game/Gameplay/Match/BP_MatchWidget.BP_MatchWidget_C" (Game|GetPlayerController 0)))
  (bind _output_get (Variables|Widgets|SetStartWidget _returnvalue))
  (UserInterface|Viewport|AddtoViewport _output_get 0))

(event EventOnMatchReady
  (CallFunction|ClearWidget)
  (bind _returnvalue (UserInterface|CreateWidget "/Game/Gameplay/Match/BP_MatchMainMenu.BP_MatchMainMenu_C" (Game|GetPlayerController 0)))
  (bind _output_get (Variables|Widgets|SetMainWidget _returnvalue))
  (UserInterface|Viewport|AddtoViewport _output_get 0))

(event EventOnSwitchRound
  (if (Variables|Default|GetbPlayerRound)
    (Utilities|FlowControl|Delay 0.3)
    (Game|Feedback|ClientStartCameraShake (Game|GetPlayerController 0) "/Game/Gameplay/Match/BP_RoundSwitchShake.BP_RoundSwitchShake_C" (/ 5.0 (Variables|Default|GetCurrentRoundTime)) "CameraLocal" "0, 0, 0")))

(fn ConstructionScript)

(fn ClearWidget
  (bind _finishwidget (Variables|Widgets|GetFinishWidget))
  (bind _startwidget (Variables|Widgets|GetStartWidget))
  (bind _mainwidget (Variables|Widgets|GetMainWidget))
  (Utilities|FlowControl|Sequence
    (:then_0
      (Utilities|IsValid _startwidget
        (:Is%20Valid
          (Widget|RemovefromParent _startwidget))))
    (:then_1
      (Utilities|IsValid _finishwidget
        (:Is%20Valid
          (Widget|RemovefromParent _finishwidget))))
    (:then_2
      (Utilities|IsValid _mainwidget
        (:Is%20Valid
          (Widget|RemovefromParent _mainwidget))))))